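; BP_platform is a moving platform that shuttles endlessly between its starting transform and an offset Destination location and rotation.
; BeginPlay caches the Platform component's relative transform and scales the Animator timeline's play rate by the inverse of TravelTimeInSeconds.
; The timeline's alpha drives position and rotation lerps.
; On each finish, it waits PauseTime, then a FlipFlop alternates between reversing and replaying the timeline.
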(event Custom|Start%20Movement
  (bind _destination (Variables|Default|GetDestination))
  (bind _initial_position (Variables|Default|GetInitial%20Position))
  (bind _initial_rotation (Variables|Default|GetInitial%20Rotation))
  (bind _alpha (Timeline|Animator Play)
    (:Update
      (Variables|Default|SetLerpAlpha _alpha)
      ;[1 1 1] Move the platform
      (Transformation|SetRelativeLocationAndRotation (Variables|Default|GetPlatform) (Math|Vector|Lerp(Vector) _initial_position (+ _initial_position (.location _destination)) (Variables|Default|GetLerpAlpha)) (Math|Rotator|Lerp(Rotator) _initial_rotation (Math|Rotator|CombineRotators _initial_rotation (.rotation _destination)) (Variables|Default|GetLerpAlpha)) false false))
    (:Finished
      ;[1 1 1] Pause and determine next action
      (Utilities|FlowControl|Delay (Variables|Default|GetPause%20time))
      (Utilities|FlowControl|FlipFlop
        (:A
          (CallFunction|ReverseMovement))
        (:B
          (CallFunction|StartMovement))))))

(event Custom|Reverse%20Movement
  (bind _destination (Variables|Default|GetDestination))
  (bind _initial_position (Variables|Default|GetInitial%20Position))
  (bind _initial_rotation (Variables|Default|GetInitial%20Rotation))
  (bind _alpha (Timeline|Animator Reverse)
    (:Update
      (Variables|Default|SetLerpAlpha _alpha)
      ;[1 1 1] Move the platform
      (Transformation|SetRelativeLocationAndRotation (Variables|Default|GetPlatform) (Math|Vector|Lerp(Vector) _initial_position (+ _initial_position (.location _destination)) (Variables|Default|GetLerpAlpha)) (Math|Rotator|Lerp(Rotator) _initial_rotation (Math|Rotator|CombineRotators _initial_rotation (.rotation _destination)) (Variables|Default|GetLerpAlpha)) false false))
    (:Finished
      ;[1 1 1] Pause and determine next action
      (Utilities|FlowControl|Delay (Variables|Default|GetPause%20time))
      (Utilities|FlowControl|FlipFlop
        (:A
          (CallFunction|ReverseMovement))
        (:B
          (CallFunction|StartMovement))))))

(event EventBeginPlay
  (bind _platform (Variables|Default|GetPlatform))
  (bind _returnvalue (Transformation|GetRelativeTransform _platform))
  ;[1 1 1] Store Start Position
  (Variables|Default|SetInitial%20Position (.location _returnvalue))
  (Variables|Default|SetInitial%20Rotation (.rotation _returnvalue))
  ;[1 1 1] Scale Playback with Travel time speed
  (Components|Timeline|SetPlayRate (Variables|Default|GetAnimator) (/ 1.0 (Variables|Default|GetTravelTimeInSeconds)))
  (CallFunction|StartMovement))

(fn ConstructionScript)